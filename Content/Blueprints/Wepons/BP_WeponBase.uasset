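; Base weapon Blueprint that deals hitscan damage to enemies.
; On BeginPlay it caches the third-person player character as the attack originator.
; DoAttack line-traces 1000 units forward from the static mesh on Visibility with persistent debug drawing, sending TakeDamageMessage to hit actors implementing BPI_Enemy.
; An AttackRate Delay follows damage or a miss, but nothing runs after it.
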(event `self.ReceiveBeginPlay`
  (bind _asbp_third_person_character (cast `/Game/ThirdPerson/Blueprints/BP_ThirdPersonCharacter` (`GameplayStatics.GetPlayerCharacter` 0)))
  (set `self.PlayerRef` _asbp_third_person_character)
  (`KismetSystemLibrary.PrintString` "Hello"))

(event `/Game/Blueprints/Wepons/BPI_Weapon.DoAttack`
  (bind _outhit (`self.TraceAttack`))
  (bind (_bblockinghit _binitialoverlap _time _distance _location _impactpoint _normal _impactnormal _physmat _hitactor) (`GameplayStatics.BreakHitResult` _outhit))
  (if _bblockinghit
    (if (`KismetSystemLibrary.DoesImplementInterface` _hitactor "/Game/Enemy/BPI_Enemy.BPI_Enemy_C")
      (message `/Game/Enemy/BPI_Enemy.TakeDamage` _hitactor (`self.Damage`) (`self.PlayerRef`))
      (`KismetSystemLibrary.Delay` (`self.AttackRate`) :!label _label))
    (else
      (goto _label))))

(fn `TraceAttack`
  (returns (OutHit :type "HitResult Structure"))
  (bind _staticmesh (`self.StaticMesh`))
  (bind _returnvalue (`SceneComponent.K2_GetComponentLocation` _staticmesh))
  (bind _outhit (`KismetSystemLibrary.LineTraceSingle` :`Start` _returnvalue :`End` (+ _returnvalue (* (`SceneComponent.GetForwardVector` _staticmesh) 1000.0)) :`TraceChannel` "TraceTypeQuery1" :`DrawDebugType` "Persistent"))
  (return _outhit))

(fn `UserConstructionScript`)
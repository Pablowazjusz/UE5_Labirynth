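; CLM_Camera is a placed camera actor that becomes the player's view when the player enters its StartTrigger volume, or at BeginPlay if flagged as the default camera.
; Each switch calls SetViewTargetWithBlend and passes its camera component to the player character through an interface message.
; View-target events track whether it is active, and while active with FocusOnPlayer set, Tick rotates the camera to look at the player.
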(event `self.ReceiveBeginPlay`
  (if (`self.DefaultCamera`)
    (`PlayerController.SetViewTargetWithBlend` (`GameplayStatics.GetPlayerController` 0) self 0.0 "VTBlend_Linear" 0.0 false)
    (message `/Game/ThirdPerson/Blueprints/BPI_Player.UpdateCameraComponent` (`GameplayStatics.GetPlayerCharacter` 0) (`self.Camera`) :!label _label)))

(event `self.StartTrigger.OnComponentBeginOverlap`
  (params (OverlappedComponent :type "PrimitiveComponent Object Reference") (OtherActor :type "Actor Object Reference") (OtherComp :type "PrimitiveComponent Object Reference") (OtherBodyIndex :type Integer) (bFromSweep :type Boolean) (SweepResult :type "HitResult Structure (by ref)"))
  (bind _yes (message `/Game/ThirdPerson/Blueprints/BPI_Player.isPlayer` OtherActor))
  (if _yes
    (`PlayerController.SetViewTargetWithBlend` (`GameplayStatics.GetPlayerController` 0) self 0.0 "VTBlend_Linear" 0.0 true)
    (goto _label)))

(event `self.K2_OnBecomeViewTarget`
  (params (PC :type "PlayerController Object Reference"))
  (set `self.ActiveCamera` true))

(event `self.K2_OnEndViewTarget`
  (params (PC :type "PlayerController Object Reference"))
  (set `self.ActiveCamera` false))

(event `self.ReceiveTick`
  (params (DeltaSeconds :type "Float (single-precision)"))
  (if (and (`self.ActiveCamera`) (`self.FocusOnPlayer`))
    (`SceneComponent.K2_SetWorldRotation` (`self.Camera`) (`KismetMathLibrary.FindLookAtRotation` (`SceneComponent.K2_GetComponentLocation` (`self.Camera`)) (`self.K2_GetActorLocation` (`GameplayStatics.GetPlayerCharacter` 0))) false false)))

(fn `isPlayer`
  (returns (Yes :type Boolean))
  (return false))

(fn `UserConstructionScript`)
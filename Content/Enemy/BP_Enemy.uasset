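; Zombie enemy character that roams, chases the player on sight, attacks in melee and ragdolls when its health runs out.
; A recursive AI Move To wanders between random reachable points, while Pawn Sensing starts the chase and a retriggerable delay resumes roaming after sightings stop.
; Attacks halt movement, play a montage and apply delayed sphere-overlap damage, gated by CanAttack and a DoOnce.
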(event `EnemyDeath`
  (`PrimitiveComponent.SetSimulatePhysics` (`self.Mesh`) true)
  (`PrimitiveComponent.SetCollisionEnabled` (`self.Mesh`) "PhysicsOnly")
  (`PrimitiveComponent.SetCollisionEnabled` (`self.CapsuleComponent`) "NoCollision")
  (set `self.EnemyHealth` 0.0)
  (`CharacterMovementComponent.DisableMovement` (`self.CharacterMovement`)))

(event `/Game/Enemy/BPI_Enemy.TakeDamage`
  (params (Damage :type "Float (double-precision)") (AttackOriginator :type "Actor Object Reference"))
  ;[1 1 1] Damage
  (`KismetSystemLibrary.PrintString` (`KismetStringLibrary.Conv_DoubleToString` Damage))
  (bind _output_get (set `self.EnemyHealth` (`KismetMathLibrary.FClamp` (- (`self.EnemyHealth`) Damage) 0.0 (`self.EnemyMaxHealth`))))
  (if (<= _output_get 0.0)
    (`/Engine/EditorBlueprintResources/StandardMacros.IsValid` self
      (:`Is Valid`
        (`self.EnemyDeath`)))))

(event `self.ReceiveBeginPlay`
  (`self.EnemyRoam`))

(event `EnemyRoam`
  ;[1 1 1] Patrol
  (`|AIMoveTo` self (`NavigationSystemV1.K2_GetRandomReachablePointInRadius` (`self.K2_GetActorLocation`) 1500.0 null null) null
    (:`OnSuccess`
      (`KismetSystemLibrary.Delay` (`KismetMathLibrary.RandomFloat`))
      (`self.EnemyRoam`))))

(event `self.PawnSensing.OnSeePawn`
  (params (Pawn :type "Pawn Object Reference"))
  ;[1 1 1] Chase
  (set `self.CanAttack` true)
  (`|ExecutionSequence`
    (:`then_0`
      (`|AIMoveTo` self (0.0 0.0 0.0) (`GameplayStatics.GetPlayerCharacter` 0) 70.0
        (:`OnSuccess`
          (if (`self.CanAttack`)
            (set `self.CanAttack` false)
            (`self.Attack`)))))
    (:`then_1`
      (`KismetSystemLibrary.RetriggerableDelay` 1.0)
      (`self.EnemyRoam`))))

(event `Attack`
  (`CharacterMovementComponent.DisableMovement` (`self.CharacterMovement`))
  (`/Engine/EditorBlueprintResources/StandardMacros.DoOnce` false :!label _label
    (:`Completed`
      (bind _returnvalue (`self.PlayAnimMontage` "/Game/Enemy/zombie/Zombie_Attack__1__Montage.Zombie_Attack__1__Montage"))
      (`KismetSystemLibrary.Delay` 1.0)
      (bind _outactors (`KismetSystemLibrary.SphereOverlapActors` (`SceneComponent.K2_GetComponentLocation` (`self.Damage`)) 100.0 (`self.Object Types`)))
      (for _array_element _outactors
        (`GameplayStatics.ApplyDamage` _array_element 0.2))
      (`KismetSystemLibrary.Delay` _returnvalue)
      (set `self.CanAttack` true)
      (`CharacterMovementComponent.SetMovementMode` (`self.CharacterMovement`) "MOVE_Walking" 0)
      (goto _label :!via `Reset`))))

(fn `UserConstructionScript`)